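; BP_actor is an actor that travels along a spline path placed in the level, starting automatically on BeginPlay.
; It finds a BP_path actor by class, stores it as Path, and calls StartMoving to play a Timeline.
; Each Timeline update lerps the Alpha across the spline length and sets the actor's world location and rotation from the spline transform at that distance.
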(event `self.ReceiveBeginPlay`
  (bind _returnvalue (`GameplayStatics.GetActorOfClass` "/Game/Kobo_ForestVillage/Meshes/BP_path.BP_path_C"))
  (set `self.Path` _returnvalue)
  (`self.startMoving`))

(event `startMoving`
  (bind (_direction _alpha) (`Timeline|Timeline`)
    (:`Update`
      (bind (_returnvalue_location _returnvalue_rotation) (`KismetMathLibrary.BreakTransform` (`SplineComponent.GetTransformAtDistanceAlongSpline` (`/Game/Kobo_ForestVillage/Meshes/BP_path.Spline` (`self.Path`)) (`KismetMathLibrary.Lerp` 0.0 (`SplineComponent.GetSplineLength` (`/Game/Kobo_ForestVillage/Meshes/BP_path.Spline` (`self.Path`))) _alpha) "World" false)))
      (`self.K2_SetActorLocationAndRotation` _returnvalue_location _returnvalue_rotation))))

(fn `UserConstructionScript`)